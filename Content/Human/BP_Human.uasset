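; BP_Human is a human that turns into a zombie when it takes any damage.
; On authority, the first hit sets IsInfected, notifies BP_TopDownGameMode that a human died, and spawns a BP_Zombie at the human's transform before destroying the human.
; If the spawned zombie is invalid, the graph loops back, repeating both the death notification and the spawn.
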(event `self.ReceiveAnyDamage`
  (params (Damage :type "Float (single-precision)") (DamageType :type "DamageType Object Reference") (InstigatedBy :type "Controller Object Reference") (DamageCauser :type "Actor Object Reference"))
  (`KismetSystemLibrary.PrintString` "DIeeeeeeeeeeeeeeeeeeeeeeeeeeeeeeeeeeeeeeeeeeeeeeeeeeeeeeeeee")
  (`/Engine/EditorBlueprintResources/ActorMacros.Switch Has Authority`
    (:`Authority`
      (if (not (`self.IsInfected`))
        (set `self.IsInfected` true :!label _label)
        (bind _asbp_top_down_game_mode (cast `/Game/TopDown/Blueprints/BP_TopDownGameMode` (`GameplayStatics.GetGameMode`)))
        (`/Game/TopDown/Blueprints/BP_TopDownGameMode.Event_OnHumanDied` _asbp_top_down_game_mode)
        (bind _returnvalue (`|SpawnActorFromClass` "/Game/Zombie/BP_Zombie.BP_Zombie_C" (`self.GetTransform`) "AdjustIfPossibleButAlwaysSpawn" "MultiplyWithRoot" null null))
        (`/Engine/EditorBlueprintResources/StandardMacros.IsValid` _returnvalue
          (:`Is Valid`
            (`self.K2_DestroyActor`))
          (:`Is Not Valid`
            (goto _label)))))))

(fn `UserConstructionScript`)